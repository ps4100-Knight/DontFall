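; BP_GargoyleSwitch is a switch Blueprint whose light turns on once it is activated.
; BeginPlay sets the Light intensity to zero, and Tick polls IsActivated every frame, raising the intensity to full brightness while it is true.
; Nothing in these graphs sets IsActivated or dims the light again, and the overlap event is a disabled stub.
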(event EventBeginPlay
  (|CallParentFunction)
  (Rendering|Components|Light|SetIntensity (Variables|Default|GetLight) 0.0))

(event Collision|EventActorBeginOverlap
  (params (OtherActor :type Actor%20Object%20Reference))
  (|CallParentFunction OtherActor) ; This node is disabled and will not be called.\nDrag off pins to build functionality.
)

(event EventTick
  (params (DeltaSeconds :type Float%20%28single-precision%29))
  (|CallParentFunction DeltaSeconds)
  (if (Variables|Default|GetIsActivated)
    (Rendering|Components|Light|SetIntensity (Variables|Default|GetLight) 5e+03)))

(fn ConstructionScript
  (|CallParentFunction))