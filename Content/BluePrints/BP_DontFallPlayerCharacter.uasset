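; Player character Blueprint that handles interaction with gargoyle switches and works around a collision glitch.
; On Interact press, it queries the Interactor for a target and, if that is a BP_GargoyleSwitch, sets it activated.
; Every Tick, it sweeps the movement component slightly out and back to the same location, forcing collision checks while the net position stays unchanged.
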(event EventBeginPlay)

(event Collision|EventActorBeginOverlap
  (params (OtherActor :type Actor%20Object%20Reference)))

(event EventTick
  (params (DeltaSeconds :type Float%20%28single-precision%29))
  (bind _returnvalue (Transformation|GetActorRotation))
  (bind _charactermovement (Variables|Character|GetCharacterMovement))
  ;[1 1 1] To fix the collision glitch, makes the character move and come back to same location every tick and in the process makes it check for collisions
  (Class|MovementComponent|MoveUpdatedComponent _charactermovement "1.000000,1.000000, 0" _returnvalue true)
  (Class|MovementComponent|MoveUpdatedComponent _charactermovement "-1.000000,-1.000000, 0" _returnvalue true))

(event Input|ActionEvents|InputActionInteract
  (params (Key :type Key%20Structure :default "None"))
  (:Pressed
    (bind _hitactor (Class|Interactor|Interaction (Variables|Default|GetInteractor)))
    (bind _asbp_gargoyle_switch (Utilities|Casting|CastToBP_GargoyleSwitch _hitactor))
    (Variables|/Script/DontFallCPP.Switch|SetIsActivated _asbp_gargoyle_switch true)))

(fn ConstructionScript
  (|CallParentFunction))